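; TombManager sets up a Minesweeper-style layout across the level's Tomb actors when play begins.
; It gathers every Tomb, then puts enemies in randomly indexed ones, with no check against repeat picks.
; Each tomb left empty then counts the occupied tombs in its Vecinos (neighbors) list and receives that total through SetNearbyNumbers.
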(event `self.ReceiveBeginPlay`
  (bind _outactors (`GameplayStatics.GetAllActorsOfClass` "/Game/Blueprints/Tomb.Tomb_C"))
  (for _array_element _outactors
    (`KismetArrayLibrary.Array_Add` (`self.tombs`) _array_element))
  (for _ (range (+ (`self.numberOfFullTombs`) 1))
    (`/Game/Blueprints/Tomb.SetEnemy` (`KismetArrayLibrary.Array_Get` (`self.tombs`) (`KismetMathLibrary.RandomIntegerInRange` 0 (`KismetArrayLibrary.Array_Length` (`self.tombs`)))) 1))
  (for _array_element_2 (`self.tombs`)
    (if (== (`/Game/Blueprints/Tomb.enemyInside` _array_element_2) 0)
      (set `self.acu` 0)
      (for _array_element_3 (`/Game/Blueprints/Tomb.vecinos` _array_element_2)
        (if (!= (`/Game/Blueprints/Tomb.enemyInside` _array_element_3) 0)
          (set `self.acu` (+ (`self.acu`) 1))))
      (`/Game/Blueprints/Tomb.SetNearbyNumbers` _array_element_2 (`self.acu`)))))

(event `self.ReceiveActorBeginOverlap`
  (params (OtherActor :type "Actor Object Reference")))

(event `self.ReceiveTick`
  (params (DeltaSeconds :type "Float (single-precision)")))

(fn `UserConstructionScript`)