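; Door actor (Puerta) that gates entry to the Catacumbas level until the player has captured a soul.
; On overlap, it reads the soul counter (ContadorAlmas) from the player's FirstPersonCharacterBP.
; At zero, it pauses the game, shows a Dialog widget with a Spanish warning in UI-only input and plays a boss voice sound.
; Otherwise, it opens the level by name.
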(event `self.ReceiveBeginPlay`)

(event `self.ReceiveActorBeginOverlap`
  (params (OtherActor :type "Actor Object Reference"))
  (bind _returnvalue (`GameplayStatics.GetPlayerController` 0))
  (bind _asfirst_person_character_bp (cast `/Game/FirstPersonBP/Blueprints/FirstPersonCharacterBP` (`GameplayStatics.GetPlayerCharacter` 0)))
  (if (== (`/Game/FirstPersonBP/Blueprints/FirstPersonCharacterBP.contadorAlmas` _asfirst_person_character_bp) 0)
    (`GameplayStatics.SetGamePaused` true)
    (bind _returnvalue_2 (`|CreateWidget` "/Game/UI/Dialog.Dialog_C"))
    (`UserWidget.AddToViewport` _returnvalue_2 0)
    (set `PlayerController.bShowMouseCursor` true _returnvalue)
    (`WidgetBlueprintLibrary.SetInputMode_UIOnlyEx` _returnvalue)
    (`KismetArrayLibrary.Array_Add` (`/Game/UI/Dialog.textToShow` _returnvalue_2) "Necesitas capturar un alma antes de abrir la puerta")
    (`GameplayStatics.PlaySound2D` "/Game/Sounds/boss_speak.boss_speak")
    (else
      (`GameplayStatics.OpenLevel` "Catacumbas"))))

(event `self.ReceiveTick`
  (params (DeltaSeconds :type "Float (single-precision)")))

(fn `UserConstructionScript`)