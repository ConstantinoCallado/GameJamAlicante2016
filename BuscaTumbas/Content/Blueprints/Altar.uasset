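; Altar actor that introduces the necromancy gameplay (dig for graves, raise the dead, harvest souls for resurrection) when the player overlaps it.
; The overlap pauses the game, switches to UI-only input with a cursor, and queues Spanish tutorial lines in a Dialog widget.
; It then calls PickUpGear on the first-person character and hides the referenced shovel and book meshes.
; No guard prevents the sequence from repeating on later overlaps.
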(event `self.ReceiveBeginPlay`)

(event `self.ReceiveActorBeginOverlap`
  (params (OtherActor :type "Actor Object Reference"))
  (bind _returnvalue (`GameplayStatics.GetPlayerController` 0))
  (if (`self.ActorHasTag` OtherActor "Player")
    (`GameplayStatics.SetGamePaused` true)
    (bind _returnvalue_2 (`|CreateWidget` "/Game/UI/Dialog.Dialog_C"))
    (`UserWidget.AddToViewport` _returnvalue_2 0)
    (set `PlayerController.bShowMouseCursor` true _returnvalue)
    (`WidgetBlueprintLibrary.SetInputMode_UIOnlyEx` _returnvalue)
    (bind _texttoshow (`/Game/UI/Dialog.textToShow` _returnvalue_2))
    (`KismetArrayLibrary.Array_Add` _texttoshow "Has sido bendecido con la marca del renacimiento, esto te concede otra oportunidad para volver de entre los muertos. \n \nTe concederé acceso al libro de la nigromancia, tu resurgimiento tiene un coste, segar las almas de los muertos, ¡álzalos y canaliza sus almas en tí!")
    (`KismetArrayLibrary.Array_Add` _texttoshow "Primero debes encontrar las tumbas de los caídos con la ayuda de tu pala [CLICK IZQUIERDO], cava poco a poco y permanece atento a los símbolos.  \n \n¡CUIDADO! Si usas la pala sobre una tumba llena destruirás los restos del humano.")
    (`KismetArrayLibrary.Array_Add` _texttoshow "Una vez hayas localizado una tumba llena, usa tu libro para lanzar un hechizo de nigromancia sobre ella [CLICK DERECHO]. \n¡Cuando el saco de huesos se levante destrúyelo con tu pala para robar su alma! \n \n¡CUIDADO! Los hechizos de nigromancia necesitan almas para ser usados, no los emplees a la ligera.")
    (`KismetArrayLibrary.Array_Add` _texttoshow "Cuando tengas las necesarias tu marca brillará de nuevo, vuelve a mí y te daré la vida de nuevo!")
    (bind _asfirst_person_character_bp (cast `/Game/FirstPersonBP/Blueprints/FirstPersonCharacterBP` (`GameplayStatics.GetPlayerCharacter` 0)))
    (`/Game/FirstPersonBP/Blueprints/FirstPersonCharacterBP.PickUpGear` _asfirst_person_character_bp)
    (`SceneComponent.SetVisibility` (`StaticMeshActor.StaticMeshComponent` (`self.palaRef`)) false false)
    (`SceneComponent.SetVisibility` (`StaticMeshActor.StaticMeshComponent` (`self.libroRef`)) false false)))

(event `self.ReceiveTick`
  (params (DeltaSeconds :type "Float (single-precision)")))

(fn `UserConstructionScript`)