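; Fatuo is an actor that hovers by bobbing up and down around its starting height.
; BeginPlay stores the initial Z as BaseZ.
; Tick sets the location from the current X and Y plus a sine of game time added to BaseZ, so the motion follows absolute time rather than accumulated offsets.
; The overlap event and construction script are empty.
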(event `self.ReceiveBeginPlay`
  (bind (_returnvalue_x _returnvalue_y _returnvalue_z) (`KismetMathLibrary.BreakVector` (`self.K2_GetActorLocation`)))
  (set `self.baseZ` _returnvalue_z))

(event `self.ReceiveActorBeginOverlap`
  (params (OtherActor :type "Actor Object Reference")))

(event `self.ReceiveTick`
  (params (DeltaSeconds :type "Float (single-precision)"))
  (bind (_returnvalue_x _returnvalue_y) (`KismetMathLibrary.BreakVector` (`self.K2_GetActorLocation`)))
  (`self.K2_SetActorLocation` (`KismetMathLibrary.MakeVector` _returnvalue_x _returnvalue_y (+ (* (`KismetMathLibrary.Sin` (* (`KismetSystemLibrary.GetGameTimeInSeconds`) 2.0)) 15.0) (`self.baseZ`)))))

(fn `UserConstructionScript`)