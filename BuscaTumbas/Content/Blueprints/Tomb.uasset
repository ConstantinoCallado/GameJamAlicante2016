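; Tomb is a diggable grave actor in what appears to be a Minesweeper-style grid, holding either a hidden enemy or a nearby-count number.
; The construction script caches neighboring tombs in Vecinos through a sphere overlap.
; SetEnemy and SetNearbyNumbers reveal the matching bones or number components.
; Cavar digs once, removing the gravel with particles and, if an enemy is inside, adding bones to the player character.
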(event `self.ReceiveBeginPlay`)

(event `self.ReceiveActorBeginOverlap`
  (params (OtherActor :type "Actor Object Reference")))

(fn `Cavar`
  (`/Engine/EditorBlueprintResources/StandardMacros.DoOnce` false
    (:`Completed`
      (`KismetSystemLibrary.PrintString` "Sonido cavar")
      (`PrimitiveComponent.SetCollisionEnabled` (`self.TombGravel`) "NoCollision")
      (`ActorComponent.Activate` (`self.DigParticles`) false)
      (`ActorComponent.K2_DestroyComponent` (`self.TombGravel`))
      (if (> (`self.enemyInside`) 0)
        (`ActorComponent.Activate` (`self.DigBone`) false)
        (bind _asfirst_person_character_bp (cast `/Game/FirstPersonBP/Blueprints/FirstPersonCharacterBP` (`GameplayStatics.GetPlayerCharacter` 0)))
        (`/Game/FirstPersonBP/Blueprints/FirstPersonCharacterBP.AddBones` _asfirst_person_character_bp 15)
        (`KismetSystemLibrary.PrintString` "Sonido ERROR")))))

(fn `SetEnemy`
  (params (enemyType :type Integer))
  (set `self.enemyInside` enemyType)
  (`SceneComponent.SetVisibility` (`self.bones`) true false))

(fn `SetNearbyNumbers`
  (params (number :type Integer))
  (switch `int` number
    (:`1`
      (`SceneComponent.SetVisibility` (`self.one`) true false))
    (:`2`
      (`SceneComponent.SetVisibility` (`self.two`) true false))
    (:`3`
      (`SceneComponent.SetVisibility` (`self.three`) true false))
    (:`4`
      (`SceneComponent.SetVisibility` (`self.four`) true false))
    (:`5`
      (`SceneComponent.SetVisibility` (`self.five`) true false))))

(fn `UserConstructionScript`
  (`KismetArrayLibrary.Array_Clear` (`self.vecinos`))
  (bind _outactors (`KismetSystemLibrary.SphereOverlapActors_NEW` (`self.K2_GetActorLocation`) 300.0 (`|MakeArray` "ObjectTypeQuery2" :!type "EObjectTypeQuery Enum") "Tomb_C" (`|MakeArray` self :!type "Actor Object Reference")))
  (for _array_element _outactors
    (bind _astomb (cast `/Game/Blueprints/Tomb` _array_element))
    (`KismetArrayLibrary.Array_Add` (`self.vecinos`) _astomb)))